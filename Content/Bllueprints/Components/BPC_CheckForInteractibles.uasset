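; Actor component that finds the puzzle interactable a player-controlled pawn is looking at and highlights it.
; Each tick it sphere-traces on Visibility from the camera along its forward vector, with debug drawing on.
; A hit that implements BPI_Puzzle and reports itself interactable becomes CurrentInteractible, moving the highlight when the target changes.
; Otherwise it clears the highlight and still stores the hit actor as CurrentInteractible.
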(event EventBeginPlay)

(event EventTick
  (params (DeltaSeconds :type Float%20%28single-precision%29))
  (bind _camera (Variables|Default|GetCamera))
  (bind _returnvalue (Transformation|GetWorldLocation _camera))
  (bind _outhit (Collision|SphereTraceByChannel _returnvalue (+ _returnvalue (* (Math|Vector|GetForwardVector _camera) (Variables|Default|GetInteractionDistance))) (Variables|Default|GetInteractionRadius) "TraceTypeQuery1" false 0 "ForDuration" true "(R=1.000000,G=0.000000,B=0.000000,A=1.000000)" "(R=0.000000,G=1.000000,B=0.000000,A=1.000000)" 0.1))
  (bind _isinteractable (Class|BPIPuzzle|IsInteractable(Message) (.HitActor (Collision|BreakHitResult _outhit))))
  (if (Math|Boolean|ANDBoolean _isinteractable (Utilities|DoesObjectImplementInterface (.HitActor (Collision|BreakHitResult _outhit)) "/Game/Bllueprints/Interfaces/BPI_Puzzle.BPI_Puzzle_C") (Pawn|IsPlayerControlled (.AsPawn (Utilities|Casting|CastToPawn (Components|GetOwner)))))
    (if (not (== (.HitActor (Collision|BreakHitResult _outhit)) (Variables|Default|GetCurrentInteractible)))
      (Class|BPIPuzzle|SetHighlight(Message) (Variables|Default|GetCurrentInteractible) false)
      (bind _output_get (Variables|Default|SetCurrentInteractible (.HitActor (Collision|BreakHitResult _outhit))))
      (Class|BPIPuzzle|SetHighlight(Message) _output_get true))
    (else
      (Class|BPIPuzzle|SetHighlight(Message) (Variables|Default|GetCurrentInteractible) false)
      (Variables|Default|SetCurrentInteractible (.HitActor (Collision|BreakHitResult _outhit))))))