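; BP_InteractPad is an interactable pad actor that animates its static mesh when interacted with and can show a highlight.
; Interact plays the Doorpad timeline at a raised play rate, interpolating the mesh's relative X location by one unit.
; SetHighlight toggles the M_TextureWave overlay material on the mesh.
; IsInteractable always returns false, and the construction script is empty.
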(event EventBeginPlay)

(event EventSetHighlight
  (params (Show :type Boolean))
  (Rendering|Material|SetOverlayMaterial (Variables|Default|GetStaticMesh) (select Show "/Game/Materials/Overlay/M_TextureWave.M_TextureWave" 0) :!class /Script/Engine.MeshComponent))

(event EventInteract
  (params (LastPossess :type Pawn%20Object%20Reference))
  (Components|Timeline|SetPlayRate (Variables|Default|GetDoorpad) 4.0)
  (bind _newtrack_0 (Timeline|Doorpad Play)
    (:Update
      (Transformation|SetRelativeLocation (Variables|Default|GetStaticMesh) (Math|Vector|MakeVector (Math|Float|Lerp 0.0 1.0 _newtrack_0) 0.0 0.0) false false))))

(fn ConstructionScript)

(fn IsInteractable
  (return false))