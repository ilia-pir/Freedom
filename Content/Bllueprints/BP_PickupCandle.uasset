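; BP_PickupCandle is an interactable, possessable candle that the player can highlight, pick up, drop and inspect.
; Interact delegates pickup to BP_Player, while Drop detaches it and timeline-lerps it to the target transform before re-enabling collision.
; Inspection possesses the candle, matches its camera to the player's and lerps InspectPivot to the player's inspect point.
; IMC_Pickup is active while possessed for look-driven rotation and backing out, which reverses the timeline.
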(event Custom|Drop
  (params (NewLocation :type Vector) (NewRotation :type Rotator))
  (Transformation|DetachFromActor "KeepWorld" "KeepRelative" "KeepRelative")
  (Variables|/Game/Bllueprints/BP_Player.BP_Player_C|SetObject%20In%20Hand (Variables|Data|GetPlayer) 0)
  (Variables|Data|SetHold%20Transform (Transformation|GetActorTransform))
  (bind _alpha (Timeline|DropTimeline PlayFromStart)
    (:Update
      (Transformation|SetActorLocationAndRotation (Math|Vector|Lerp(Vector) (.location (Variables|Data|GetHold%20Transform)) NewLocation _alpha) (Math|Rotator|Lerp(Rotator) (.rotation (Variables|Data|GetHold%20Transform)) NewRotation _alpha)))
    (:Finished
      (Collision|SetActorEnableCollision true))))

(event Custom|Stop%20Inspect
  (if (not (Audio|Components|Audio|IsPlaying (Variables|Default|GetInspecttimeline)))
    (Utilities|MySmoothPossess (Variables|Data|GetPlayer) 0.0)
    (Variables|Data|SetRelative%20Rotation (Variables|/Script/Engine.SceneComponent|GetRelativeRotation (Variables|Default|GetinspectPivot)))
    (CallFunction|ReverseInspect)))

(event Custom|ReverseInspect
  (bind _alpha (Timeline|InspectTimeline ReverseFromEnd)
    (:Update
      (Transformation|SetRelativeLocation (Variables|Default|GetinspectPivot) (Math|Vector|Lerp(Vector) (Variables|Data|GetInhandLocation) (Math|Transform|InverseTransformLocation (Transformation|GetActorTransform) (Transformation|GetWorldLocation (Variables|/Game/Bllueprints/BP_Player.BP_Player_C|GetInspect%20Location (Variables|Data|GetPlayer)))) _alpha) false false)
      (Transformation|SetRelativeRotation (Variables|Default|GetinspectPivot) (Math|Rotator|Lerp(Rotator) "0, 0, 0" (Variables|Data|GetRelative%20Rotation) _alpha) false false))))

(event Custom|StartInspect
  (bind _player (Variables|Data|GetPlayer))
  (bind _camera (Variables|/Game/Bllueprints/BP_Player.BP_Player_C|GetCamera _player))
  (if (and (not (Audio|Components|Audio|IsPlaying (Variables|/Game/Bllueprints/BP_Player.BP_Player_C|GetPickupTimeline (Variables|Data|GetPlayer)))) (not (Audio|Components|Audio|IsPlaying (Variables|Default|GetInspecttimeline))))
    (Variables|Data|SetInhandLocation (Variables|/Script/Engine.SceneComponent|GetRelativeLocation (Variables|Default|GetinspectPivot)))
    (Utilities|MySmoothPossess self 0.0)
    (Transformation|SetWorldLocationAndRotation (Variables|Default|GetCamera) (Transformation|GetWorldLocation _camera) (Transformation|GetWorldRotation _camera) false false)
    (bind _alpha (Timeline|InspectTimeline PlayFromStart)
      (:Update
        (Transformation|SetRelativeLocation (Variables|Default|GetinspectPivot) (Math|Vector|Lerp(Vector) (Variables|Data|GetInhandLocation) (Math|Transform|InverseTransformLocation (Transformation|GetActorTransform) (Transformation|GetWorldLocation (Variables|/Game/Bllueprints/BP_Player.BP_Player_C|GetInspect%20Location (Variables|Data|GetPlayer)))) _alpha) false false)
        (Transformation|SetRelativeRotation (Variables|Default|GetinspectPivot) (Math|Rotator|Lerp(Rotator) "0, 0, 0" (Variables|Data|GetRelative%20Rotation) _alpha) false false)))))

(event EventBeginPlay)

(event Collision|EventActorBeginOverlap
  (params (OtherActor :type Actor%20Object%20Reference)))

(event EventTick
  (params (DeltaSeconds :type Float%20%28single-precision%29)))

(event EventSetHighlight
  (params (Show :type Boolean))
  (Rendering|Material|SetOverlayMaterial (Variables|Default|GetCube) (select Show "/Game/Materials/Overlay/M_TextureWave.M_TextureWave" 0) :!class /Script/Engine.MeshComponent))

(event EventInteract
  (params (LastPossess :type Pawn%20Object%20Reference))
  (Utilities|IsValid (Variables|Data|GetPlayer)
    (:Is%20Valid
      _)
    (:Is%20Not%20Valid
      (bind _asbp_player (Utilities|Casting|CastToBP_Player LastPossess))
      (bind _output_get (Variables|Data|SetPlayer _asbp_player))))
  (Default|PickUpObject _output_get))

(event EventPossessed
  (params (NewController :type Controller%20Object%20Reference))
  (CallFunction|ChangeMappingContext false))

(event EventUnpossessed
  (params (OldController :type Controller%20Object%20Reference))
  (CallFunction|ChangeMappingContext true))

(event Input|EnhancedActionEvents|EnhancedInputActionIA_Back
  (params (ActionValue :type Boolean) (ElapsedSeconds :type Float%20%28double-precision%29) (TriggeredSeconds :type Float%20%28double-precision%29) (InputAction :type Input%20Action%20Object%20Reference :default "/Game/Inputs/Keypad/IA_Back.IA_Back"))
  (:Started
    (CallFunction|StopInspect)))

(event Input|EnhancedActionEvents|EnhancedInputActionIA_Look
  (params (ActionValue :type Vector%202D%20Structure) (ElapsedSeconds :type Float%20%28double-precision%29) (TriggeredSeconds :type Float%20%28double-precision%29) (InputAction :type Input%20Action%20Object%20Reference :default "/Game/Inputs/Playerinput/IA_Look.IA_Look"))
  (Transformation|SetRelativeRotation (Variables|Default|GetinspectPivot) (Math|Rotator|MakeRotator 0.0 (.y ActionValue) (.x ActionValue)) false false))

(fn ConstructionScript)

(fn ChangeMappingContext
  (params (Remove :type Boolean))
  (bind _returnvalue (Game|GetPlayerController 0))
  (bind _returnvalue_2 (Game|GetPlayerController 0))
  (bind _returnvalue_3 (PlayerController|LocalPlayerSubsystems|GetEnhancedInputLocalPlayerSubsystem _returnvalue))
  (bind _returnvalue_4 (PlayerController|LocalPlayerSubsystems|GetEnhancedInputLocalPlayerSubsystem _returnvalue_2))
  (if Remove
    (Utilities|IsValid _returnvalue_3
      (:Is%20Valid
        (Input|RemoveMappingContext _returnvalue_3 "/Game/Inputs/Inspect/IMC_Pickup.IMC_Pickup" "(bIgnoreAllPressedKeysUntilRelease=True,bForceImmediately=False,bNotifyUserSettings=False)")))
    (else
      (Utilities|IsValid _returnvalue_4
        (:Is%20Valid
          (Input|AddMappingContext _returnvalue_4 "/Game/Inputs/Inspect/IMC_Pickup.IMC_Pickup" 0 "(bIgnoreAllPressedKeysUntilRelease=True,bForceImmediately=False,bNotifyUserSettings=False)"))))))

(fn IsInteractable
  (return true))