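; First-person player character with movement, crouching, flashlight, pausing, interaction and carrying of a single object.
; A head-bob timeline scales with speed and fires footstep sounds chosen by a surface trace.
; A crouch timeline blends capsule height and walk speed, with uncrouching retried each tick until an overhead trace allows it.
; Pickups lerp to a spring arm and drop at a camera trace hit, while possession changes toggle the input mapping context.
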(event Custom|Head
  (bind _charactermovement (Variables|Character|GetCharacterMovement))
  (bind _velocity (Variables|/Script/Engine.MovementComponent|GetVelocity _charactermovement))
  (bind _returnvalue (Math|Vector|VectorLengthXY _velocity))
  (bind _alpha (Timeline|Timeline Play)
    (:Update
      (Components|Timeline|SetPlayRate (Variables|Default|GetTimeline) (Variables|Settings|GetHeadSpeed))
      (Transformation|SetRelativeLocation (Variables|Default|GetCamera) (Math|Vector|MakeVector 0.0 0.0 (* _alpha (Variables|Settings|GetHeadAmount) (Math|Float|MapRangeClamped _returnvalue 0.0 (Variables|Settings|GetMax%20Walk%20Speed) 0.3 1.0))) false false)
      (Variables|Settings|SetHeadSpeed (Variables|Settings|GetHeadSpeed)))
    (:EventTrack
      (if (> _returnvalue 5e+01)
        (CallFunction|PlayFootstep)))))

(event Custom|Set%20Up%20Variable
  (Utilities|FlowControl|Sequence
    (:then_0
      (Variables|Data|SetOriginal%20Height (Components|Capsule|GetUnscaledCapsuleHalfHeight (Variables|Collision|GetCapsuleComponent))))
    (:then_1
      (Variables|Settings|SetMax%20Walk%20Speed (Variables|/Script/Engine.CharacterMovementComponent|GetMaxWalkSpeed (Variables|Character|GetCharacterMovement))))))

(event Custom|Uncrouch%20Check
  (if (and (Variables|Data|GetWants%20to%20Uncrouch) (Variables|Data|GetIsCrouching))
    (CallFunction|TryUncrouching)))

(event Custom|PickUpObject
  (params (ObjectToPickup :type BP%20Pickup%20Object%20Reference))
  (Utilities|IsValid (Variables|Data|GetObject%20In%20Hand)
    (:Is%20Not%20Valid
      (bind _output_get (Variables|Data|SetObject%20In%20Hand ObjectToPickup))
      (Collision|SetActorEnableCollision _output_get false)
      (Variables|Data|SetLocation (Transformation|GetActorTransform (Variables|Data|GetObject%20In%20Hand)))
      (bind _alpha (Timeline|PickupTimeline PlayFromStart)
        (:Update
          (Transformation|SetActorTransform ObjectToPickup (Math|Transform|MakeTransform (Math|Vector|Lerp(Vector) (.location (Variables|Data|GetLocation)) (Transformation|GetWorldLocation (Variables|Default|GetSpringArmPickup)) _alpha) (Math|Rotator|Lerp(Rotator) (.rotation (Variables|Data|GetLocation)) (Transformation|GetWorldRotation (Variables|Default|GetSpringArmPickup)) _alpha true) "1.000000,1.000000,1.000000")))
        (:Finished
          (Transformation|AttachComponentToComponent (Variables|Data|GetObject%20In%20Hand) (Variables|Default|GetPickup) "None" "KeepWorld" "KeepWorld" "KeepRelative" true))))))

(event Custom|Drop%20Object
  (bind _camera (Variables|Default|GetCamera))
  (bind _returnvalue (Transformation|GetWorldLocation _camera))
  (bind (_outhit _returnvalue_2) (Collision|SphereTraceByChannel _returnvalue (+ _returnvalue (* (Math|Vector|GetForwardVector _camera) 2e+02)) 3.0 "TraceTypeQuery1" false 0 "None"))
  (if _returnvalue_2
    (Default|Drop (Variables|Data|GetObject%20In%20Hand) (.Location (Collision|BreakHitResult _outhit)) (Math|Rotator|MakeRotfromZ (.Normal (Collision|BreakHitResult _outhit))))))

(event Custom|StopHead
  (bind _charactermovement (Variables|Character|GetCharacterMovement))
  (bind _velocity (Variables|/Script/Engine.MovementComponent|GetVelocity _charactermovement))
  (bind _returnvalue (Math|Vector|VectorLengthXY _velocity))
  (bind _alpha (Timeline|Timeline Stop)
    (:Update
      (Components|Timeline|SetPlayRate (Variables|Default|GetTimeline) (Variables|Settings|GetHeadSpeed))
      (Transformation|SetRelativeLocation (Variables|Default|GetCamera) (Math|Vector|MakeVector 0.0 0.0 (* _alpha (Variables|Settings|GetHeadAmount) (Math|Float|MapRangeClamped _returnvalue 0.0 (Variables|Settings|GetMax%20Walk%20Speed) 0.3 1.0))) false false)
      (Variables|Settings|SetHeadSpeed (Variables|Settings|GetHeadSpeed)))
    (:EventTrack
      (if (> _returnvalue 5e+01)
        (CallFunction|PlayFootstep)))))

(event Custom|Stop%20Pickup
  (bind _alpha (Timeline|PickupTimeline Stop)
    (:Update
      (Transformation|SetActorTransform (stale Custom|PickUpObject ObjectToPickup) (Math|Transform|MakeTransform (Math|Vector|Lerp(Vector) (.location (Variables|Data|GetLocation)) (Transformation|GetWorldLocation (Variables|Default|GetSpringArmPickup)) _alpha) (Math|Rotator|Lerp(Rotator) (.rotation (Variables|Data|GetLocation)) (Transformation|GetWorldRotation (Variables|Default|GetSpringArmPickup)) _alpha true) "1.000000,1.000000,1.000000")))
    (:Finished
      (Transformation|AttachComponentToComponent (Variables|Data|GetObject%20In%20Hand) (Variables|Default|GetPickup) "None" "KeepWorld" "KeepWorld" "KeepRelative" true))))

(event Custom|PlayFootstep
  (bind _returnvalue (Transformation|GetActorLocation))
  (bind (_outhit _returnvalue_2) (Collision|SphereTraceByChannel _returnvalue (+ _returnvalue (* (Math|Vector|VectorDown) 1e+02)) 25.0 "TraceTypeQuery1" false 0 "None" true "(R=1.000000,G=0.000000,B=0.000000,A=1.000000)" "(R=0.000000,G=1.000000,B=0.000000,A=1.000000)" 2.0))
  (if _returnvalue_2
    (Class|FMODBlueprintStatics|PlayEventatLocation (Utilities|Select :Index (Variables|/Script/PhysicsCore.PhysicalMaterial|GetSurfaceType (.PhysMat (Collision|BreakHitResult _outhit))) :SurfaceType_Default "/Game/FMOD/Events/Footsteps.Footsteps" :SurfaceType1 "/Game/FMOD/Events/Footsteps.Footsteps" :SurfaceType2 "/Game/FMOD/Events/FootstepsCrouch.FootstepsCrouch") (Math|Conversions|ToTransform(Vector) (.Location (Collision|BreakHitResult _outhit))))))

(event EventBeginPlay
  (CallFunction|SetUpVariable)
  (CallFunction|SetupCamera)
  (CallFunction|Head))

(event EventTick
  (params (DeltaSeconds :type Float%20%28single-precision%29))
  (CallFunction|UncrouchCheck))

(event EventPossessed
  (params (NewController :type Controller%20Object%20Reference))
  (CallFunction|ChangeMappingContext false)
  (Rendering|SetVisibility (Variables|Default|GetSpotLight) (Variables|Data|GetFlashlightPrePossessed) false)
  (CallFunction|StopHead))

(event EventUnpossessed
  (params (OldController :type Controller%20Object%20Reference))
  (CallFunction|ChangeMappingContext true)
  (Variables|Data|SetFlashlightPrePossessed (Variables|/Script/Engine.SceneComponent|GetbVisible (Variables|Default|GetSpotLight)))
  (Rendering|SetVisibility (Variables|Default|GetSpotLight) (Variables|Data|GetFlashlightPrePossessed) false)
  (CallFunction|Head))

(event Custom|Try%20Uncrouching
  (bind _returnvalue (Transformation|GetActorLocation))
  ;[1 1 1] Crouch
  (bind (_outhit _returnvalue_2) (Collision|SphereTraceByChannel _returnvalue (+ _returnvalue (Math|Vector|MakeVector 0.0 0.0 (+ (Variables|Data|GetOriginal%20Height) 5.0))) (Class|CapsuleComponent|GetUnscaledCapsuleRadius (Variables|Collision|GetCapsuleComponent)) "TraceTypeQuery1" false 0 "None" true "(R=1.000000,G=0.000000,B=0.000000,A=1.000000)" "(R=0.000000,G=1.000000,B=0.000000,A=1.000000)" 0.5))
  (if (Class|KismetMathLibrary|XORBoolean (not _returnvalue_2) (== (Utilities|GetClass (.HitActor (Collision|BreakHitResult _outhit))) "/Game/Bllueprints/BP_Pickup.BP_Pickup_C"))
    (CallFunction|StopCrouching)))

(event Custom|FlashlightOff
  (bind _spotlight (Variables|Default|GetSpotLight))
  ;[1 1 1] light
  (Rendering|SetVisibility _spotlight (not (Variables|/Script/Engine.SceneComponent|GetbVisible _spotlight)) false))

(event Custom|Stop%20Crouching
  ;[1 1 1] Crouch
  (Variables|Data|SetWants%20to%20Uncrouch false)
  (Variables|Data|SetIsCrouching false)
  (bind _alpha (Timeline|Crouching Reverse)
    (:Update
      (Components|Capsule|SetCapsuleHalfHeight (Variables|Collision|GetCapsuleComponent) (Math|Float|Lerp (Variables|Data|GetOriginal%20Height) (Variables|/Script/Engine.CharacterMovementComponent|GetCrouchedHalfHeight (Variables|Character|GetCharacterMovement)) _alpha) true)
      (Variables|/Script/Engine.CharacterMovementComponent|SetMaxWalkSpeed (Variables|Character|GetCharacterMovement) (Math|Float|Lerp (Variables|Settings|GetMax%20Walk%20Speed) (Variables|/Script/Engine.CharacterMovementComponent|GetMaxWalkSpeedCrouched (Variables|Character|GetCharacterMovement)) _alpha)))))

(event Input|EnhancedActionEvents|EnhancedInputActionIA_Look
  (params (ActionValue :type Vector%202D%20Structure) (ElapsedSeconds :type Float%20%28double-precision%29) (TriggeredSeconds :type Float%20%28double-precision%29) (InputAction :type Input%20Action%20Object%20Reference :default "/Game/Inputs/Playerinput/IA_Look.IA_Look"))
  ;[1 1 1] Movement
  (Pawn|Input|AddControllerYawInput (* (.x ActionValue) (Variables|Settings|GetLookSensetivity)))
  (bind _result (Math|Float|NegateFloat (* (.y ActionValue) (Variables|Settings|GetLookSensetivity)))
    (:%20%20
      (Pawn|Input|AddControllerPitchInput _result))))

(event Input|EnhancedActionEvents|EnhancedInputActionIA_Interact
  (params (ActionValue :type Boolean) (ElapsedSeconds :type Float%20%28double-precision%29) (TriggeredSeconds :type Float%20%28double-precision%29) (InputAction :type Input%20Action%20Object%20Reference :default "/Game/Inputs/Playerinput/IA_Interact.IA_Interact"))
  (bind _checkforinteractible (Variables|Default|GetCheckForInteractible))
  ;[1 1 1] Interact
  (Utilities|IsValid (Variables|Data|GetObject%20In%20Hand)
    (:Is%20Not%20Valid
      (Utilities|IsValid _checkforinteractible
        (:Is%20Valid
          (Class|BPIPuzzle|Interact(Message) (Variables|/Game/Bllueprints/Components/BPC_CheckForInteractibles.BPC_CheckForInteractibles_C|GetCurrentInteractible _checkforinteractible) self))))))

(event Input|EnhancedActionEvents|EnhancedInputActionIA_Move
  (params (ActionValue :type Vector%202D%20Structure) (ElapsedSeconds :type Float%20%28double-precision%29) (TriggeredSeconds :type Float%20%28double-precision%29) (InputAction :type Input%20Action%20Object%20Reference :default "/Game/Inputs/Playerinput/IA_Move.IA_Move"))
  ;[1 1 1] Movement
  (Pawn|Input|AddMovementInput (Math|Vector|GetForwardVector (Math|Rotator|MakeRotator 0.0 0.0 (.yaw (Pawn|GetControlRotation :!class /Script/Engine.Pawn)))) (.x ActionValue) false)
  (Pawn|Input|AddMovementInput (Math|Vector|GetRightVector (Math|Rotator|MakeRotator 0.0 0.0 (.yaw (Pawn|GetControlRotation :!class /Script/Engine.Pawn)))) (.y ActionValue) false))

(event Input|EnhancedActionEvents|EnhancedInputActionIA_Crouch
  (params (ActionValue :type Boolean) (ElapsedSeconds :type Float%20%28double-precision%29) (TriggeredSeconds :type Float%20%28double-precision%29) (InputAction :type Input%20Action%20Object%20Reference :default "/Game/Inputs/Playerinput/IA_Crouch.IA_Crouch"))
  ;[1 1 1] Crouch
  (:Started
    (if (Variables|Data|GetIsCrouching)
      (Variables|Data|SetWants%20to%20Uncrouch true)
      (else
        (Variables|Data|SetIsCrouching true)
        (Components|Timeline|SetPlayRate (Variables|Default|GetCrouching) (Variables|Settings|GetCrouch%20Speed))
        (bind _alpha (Timeline|Crouching Play)
          (:Update
            (Components|Capsule|SetCapsuleHalfHeight (Variables|Collision|GetCapsuleComponent) (Math|Float|Lerp (Variables|Data|GetOriginal%20Height) (Variables|/Script/Engine.CharacterMovementComponent|GetCrouchedHalfHeight (Variables|Character|GetCharacterMovement)) _alpha) true)
            (Variables|/Script/Engine.CharacterMovementComponent|SetMaxWalkSpeed (Variables|Character|GetCharacterMovement) (Math|Float|Lerp (Variables|Settings|GetMax%20Walk%20Speed) (Variables|/Script/Engine.CharacterMovementComponent|GetMaxWalkSpeedCrouched (Variables|Character|GetCharacterMovement)) _alpha))))))))

(event Input|EnhancedActionEvents|EnhancedInputActionIA_Light
  (params (ActionValue :type Boolean) (ElapsedSeconds :type Float%20%28double-precision%29) (TriggeredSeconds :type Float%20%28double-precision%29) (InputAction :type Input%20Action%20Object%20Reference :default "/Game/Inputs/Playerinput/IA_Light.IA_Light"))
  (bind _spotlight (Variables|Default|GetSpotLight))
  ;[1 1 1] light
  (:Started
    (Class|FMODBlueprintStatics|PlayEvent2D "/Game/FMOD/Events/FlashLight.FlashLight")
    (Rendering|SetVisibility _spotlight (not (Variables|/Script/Engine.SceneComponent|GetbVisible _spotlight)) false)))

(event Input|EnhancedActionEvents|EnhancedInputActionIA_Drop
  (params (ActionValue :type Boolean) (ElapsedSeconds :type Float%20%28double-precision%29) (TriggeredSeconds :type Float%20%28double-precision%29) (InputAction :type Input%20Action%20Object%20Reference :default "/Game/Inputs/Playerinput/IA_Drop.IA_Drop"))
  ;[1 1 1] Drop
  (:Started
    (Utilities|IsValid (Variables|Data|GetObject%20In%20Hand)
      (:Is%20Valid
        (CallFunction|DropObject)))))

(event Input|EnhancedActionEvents|EnhancedInputActionIA_Pause
  (params (ActionValue :type Boolean) (ElapsedSeconds :type Float%20%28double-precision%29) (TriggeredSeconds :type Float%20%28double-precision%29) (InputAction :type Input%20Action%20Object%20Reference :default "/Game/Inputs/Playerinput/IA_Pause.IA_Pause"))
  (:Started
    (bind _asbp_basic (Utilities|Casting|CastToBP_Basic (Game|GetGameMode)))
    (Default|PauseGame _asbp_basic)))

(fn ConstructionScript
  (bind _returnvalue (AddComponent|AddBPCCheckforInteractibles (Variables|Default|GetCamera)))
  (Variables|Default|SetCheckForInteractible _returnvalue))

(fn ChangeMappingContext
  (params (Remove?1 :type Boolean))
  (bind _returnvalue (Game|GetPlayerController 0))
  (bind _returnvalue_2 (Game|GetPlayerController 0))
  (bind _returnvalue_3 (PlayerController|LocalPlayerSubsystems|GetEnhancedInputLocalPlayerSubsystem _returnvalue))
  (bind _returnvalue_4 (PlayerController|LocalPlayerSubsystems|GetEnhancedInputLocalPlayerSubsystem _returnvalue_2))
  (if Remove?1
    (Utilities|IsValid _returnvalue_3
      (:Is%20Valid
        (Input|RemoveMappingContext _returnvalue_3 "/Game/Inputs/Playerinput/IMC_Player.IMC_Player" "(bIgnoreAllPressedKeysUntilRelease=True,bForceImmediately=False,bNotifyUserSettings=False)")))
    (else
      (Utilities|IsValid _returnvalue_4
        (:Is%20Valid
          (Input|AddMappingContext _returnvalue_4 "/Game/Inputs/Playerinput/IMC_Player.IMC_Player" 0 "(bIgnoreAllPressedKeysUntilRelease=True,bForceImmediately=False,bNotifyUserSettings=False)"))))))

(fn SetupCamera
  (bind _returnvalue (Game|GetPlayerCameraManager 0))
  (Variables|/Script/Engine.PlayerCameraManager|SetViewPitchMin _returnvalue -6e+01)
  (Variables|/Script/Engine.PlayerCameraManager|SetViewPitchMax _returnvalue 7e+01))