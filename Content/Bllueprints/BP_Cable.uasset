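; BP_Cable is a spline-driven cable Blueprint that builds a mesh along an editable path in its construction script.
; It loops up to the spline point count, adding a spline mesh component per index with the Cable mesh and Material applied.
; Each segment takes local positions and tangents from its point and the next, so the mesh follows the curve.
; The event graph has no active logic.
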(event EventBeginPlay)

(event Collision|EventActorBeginOverlap
  (params (OtherActor :type Actor%20Object%20Reference)))

(event EventTick
  (params (DeltaSeconds :type Float%20%28single-precision%29)))

(fn ConstructionScript
  (for _index (range 0 (Spline|GetNumberOfSplinePoints (Variables|Default|GetSpline)))
    (bind _returnvalue (AddComponent|AddSplineMeshComponent false))
    (Components|StaticMesh|SetStaticMesh _returnvalue "/Game/Assets/Decoration/Cable.Cable")
    (Rendering|Material|SetMaterial _returnvalue 0 (Variables|Default|GetMaterial))
    (SplineMesh|SetStartandEnd _returnvalue (Spline|GetLocationatSplinePoint (Variables|Default|GetSpline) _index "Local") (Spline|GetTangentatSplinePoint (Variables|Default|GetSpline) _index "Local") (Spline|GetLocationatSplinePoint (Variables|Default|GetSpline) (+ _index 1) "Local") (Spline|GetTangentatSplinePoint (Variables|Default|GetSpline) (+ _index 1) "Local") true :!class /Script/Engine.SplineMeshComponent)))