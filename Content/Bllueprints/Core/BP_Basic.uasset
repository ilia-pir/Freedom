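; BP_Basic is a core Blueprint that sets up the game's UI and toggles the pause state.
; On BeginPlay it creates the root WBP_GameUI widget, adds it to the viewport and pushes the gameplay UI onto its GameplayStack.
; PauseGame pushes the pause background onto a separate PauseStack or clears that stack, switching game pause, input mode and mouse cursor visibility to match.
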(event Custom|PauseGame
  (bind _returnvalue (Game|GetPlayerController 0))
  (bind _gameui (Variables|Default|GetGameUI))
  (bind _pausestack (Variables|/Game/UI/WBP_GameUI.WBP_GameUI_C|GetPauseStack _gameui))
  (if (not (Game|IsGamePaused))
    (Class|CommonActivatableWidgetContainerBase|AddWidget _pausestack "/Game/UI/WBP_PauseBackground.WBP_PauseBackground_C")
    (Game|SetGamePaused true)
    (Input|SetInputModeUIOnly _returnvalue 0 "DoNotLock" false)
    (Variables|/Script/Engine.PlayerController|SetbShowMouseCursor _returnvalue true)
    (else
      (Class|CommonActivatableWidgetContainerBase|ClearWidgets _pausestack)
      (Game|SetGamePaused false)
      (Input|SetInputModeGameOnly _returnvalue false)
      (Variables|/Script/Engine.PlayerController|SetbShowMouseCursor _returnvalue false))))

(event EventBeginPlay
  (CallFunction|SetupUI))

(fn ConstructionScript)

(fn SetupUI
  (bind _returnvalue (UserInterface|CreateWidget "/Game/UI/WBP_GameUI.WBP_GameUI_C"))
  (bind _output_get (Variables|Default|SetGameUI _returnvalue))
  (UserInterface|Viewport|AddtoViewport _output_get 0)
  (Class|CommonActivatableWidgetContainerBase|AddWidget (Variables|/Game/UI/WBP_GameUI.WBP_GameUI_C|GetGameplayStack _output_get) "/Game/UI/WBP_GameplayUI.WBP_GameplayUI_C"))