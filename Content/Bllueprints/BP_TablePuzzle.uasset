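; BP_TablePuzzle is a table puzzle actor that reveals a text render once three slots are filled with pickups.
; Each slot collision sets its occupied flag when a BP_Pickup overlaps it, then calls a shared completion check.
; The check shows the text when all three flags are true.
; Flags never clear, as no end-overlap is handled, and any pickup fits any slot.
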(event OnComponentBeginOverlap(Slot1Collision)
  (params (OverlappedComponent :type Primitive%20Component%20Object%20Reference) (OtherActor :type Actor%20Object%20Reference) (OtherComp :type Primitive%20Component%20Object%20Reference) (OtherBodyIndex :type Integer) (bFromSweep :type Boolean) (SweepResult :type Hit%20Result%20Structure%20%28by%20ref%29))
  (Utilities|Casting|CastToBP_Pickup OtherActor)
  (Variables|Default|SetSlot1Occupied true)
  (CallFunction|CheckPuzzleCompleted))

(event OnComponentBeginOverlap(Slot2Collision)
  (params (OverlappedComponent :type Primitive%20Component%20Object%20Reference) (OtherActor :type Actor%20Object%20Reference) (OtherComp :type Primitive%20Component%20Object%20Reference) (OtherBodyIndex :type Integer) (bFromSweep :type Boolean) (SweepResult :type Hit%20Result%20Structure%20%28by%20ref%29))
  (Utilities|Casting|CastToBP_Pickup OtherActor)
  (Variables|Default|SetSlot2Occupied true)
  (CallFunction|CheckPuzzleCompleted))

(event OnComponentBeginOverlap(Slot3Collision)
  (params (OverlappedComponent :type Primitive%20Component%20Object%20Reference) (OtherActor :type Actor%20Object%20Reference) (OtherComp :type Primitive%20Component%20Object%20Reference) (OtherBodyIndex :type Integer) (bFromSweep :type Boolean) (SweepResult :type Hit%20Result%20Structure%20%28by%20ref%29))
  (Utilities|Casting|CastToBP_Pickup OtherActor)
  (Variables|Default|SetSlot3Occupied true)
  (CallFunction|CheckPuzzleCompleted))

(event Custom|CheckPuzzleCompleted
  (if (Math|Boolean|ANDBoolean (Variables|Default|GetSlot1Occupied) (Variables|Default|GetSlot2Occupied) (Variables|Default|GetSlot3Occupied))
    (Rendering|SetVisibility (Variables|Default|GetTextRender) true false)))

(event EventBeginPlay)

(event Collision|EventActorBeginOverlap
  (params (OtherActor :type Actor%20Object%20Reference)))

(event EventTick
  (params (DeltaSeconds :type Float%20%28single-precision%29)))

(fn ConstructionScript)