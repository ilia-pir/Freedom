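; BP_IP_LivingRoom is an interactable living room door pad that works once, as IsPlaying is never reset.
; Interact plays a click sound and runs the Doorpad timeline, nudging the pad mesh along local Y.
; Each timeline update also creates and plays a new LivingRoomDoor level sequence player, rather than doing so once.
; SetHighlight toggles a wave overlay material on the mesh.
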(event EventBeginPlay)

(event EventSetHighlight
  (params (Show :type Boolean))
  (Rendering|Material|SetOverlayMaterial (Variables|Default|GetStaticMesh) (select Show "/Game/Materials/Overlay/M_TextureWave.M_TextureWave" 0) :!class /Script/Engine.MeshComponent))

(event EventInteract
  (params (LastPossess :type Pawn%20Object%20Reference))
  (if (not (Variables|Default|GetIsPlaying))
    (Variables|Default|SetIsPlaying true)
    (Audio|PlaySound2D "/Engine/VREditor/Sounds/UI/Click_on_Button_Cue.Click_on_Button_Cue" 1.0 1.0 0.0 0 0)
    (Transformation|SetRelativeLocation (Variables|Default|GetStaticMesh) "0, 0, 0" false false)
    (Components|Timeline|SetPlayRate (Variables|Default|GetDoorpad) 1.0)
    (bind _newtrack_0 (Timeline|Doorpad PlayFromStart)
      (:Update
        (Transformation|SetRelativeLocation (Variables|Default|GetStaticMesh) (Math|Vector|MakeVector 0.0 (Math|Float|Lerp 0.0 1.0 _newtrack_0) 0.0) false false)
        (bind _outactor (Sequencer|Player|CreateLevelSequencePlayer "/Game/Sequences/LivingRoomDoor.LivingRoomDoor"))
        (Sequencer|Player|Play (Variables|/Script/LevelSequence.LevelSequenceActor|GetSequencePlayer _outactor) :!class /Script/MovieScene.MovieSceneSequencePlayer)))))

(fn ConstructionScript)

(fn IsInteractable
  (return true))