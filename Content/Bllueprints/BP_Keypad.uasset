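; BP_Keypad is an interactable, possessable code-entry keypad that plays a Level Sequence when the correct code is confirmed.
; Interact smooth-possesses it, and possession toggles the IMC_Keypad input context.
; Directional input moves a wrapping highlight across the button grid, while Interact animates the press and appends, confirms or cancels input.
; A correct code returns possession to the previous pawn and disables further interaction, while a wrong one shows red, then clears.
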(event Custom|ChangeButtonHighlight
  (params (Position :type Integer) (show :type Boolean))
  (Default|ButtonHighlight (Utilities|Array|Get(acopy) (Variables|Data|GetButton%20list) Position) show))

(event Custom|Exit%20Keypad
  (CallFunction|ChangeButtonHighlight (Variables|Data|GetCurrent%20Button) false)
  (Input|DisableInput 0)
  (Utilities|MySmoothPossess (Variables|Data|GetLast%20possess) 1.0)
  (Input|EnableInput 0))

(event Custom|Animate%20Press
  (Utilities|IsValid (Variables|Default|GetLastPressed)
    (:Is%20Valid
      (Transformation|SetRelativeLocation (Variables|Default|GetLastPressed) "0, 0, 0" false false))
    (:Is%20Not%20Valid
      _))
  (Variables|Default|SetLastPressed (Utilities|Array|Get(acopy) (Variables|Data|GetButton%20list) (Variables|Data|GetCurrent%20Button)))
  (Components|Timeline|SetPlayRate (Variables|Default|GetButtonAnim) 4.0)
  (bind _alpha (Timeline|ButtonAnim PlayFromStart)
    (:Update
      (Transformation|SetRelativeLocation (Variables|Default|GetLastPressed) (Math|Vector|MakeVector (Math|Float|Lerp 0.0 1.0 _alpha) 0.0 0.0) false false))))

(event EventInteract
  (params (LastPossess :type Pawn%20Object%20Reference))
  (Variables|Data|SetLast%20possess LastPossess)
  (Utilities|MySmoothPossess self 1.0)
  (bind _output_get (Variables|Data|SetCurrent%20Button 0))
  (CallFunction|ChangeButtonHighlight _output_get true))

(event EventSetHighlight
  (params (Show :type Boolean))
  (Rendering|Material|SetOverlayMaterial (Variables|Default|GetKeypad_Base) (select Show "/Game/Materials/Overlay/M_TextureWave.M_TextureWave" 0) :!class /Script/Engine.MeshComponent))

(event EventPossessed
  (params (NewController :type Controller%20Object%20Reference))
  (CallFunction|ChangeMappingContest false))

(event EventUnpossessed
  (params (OldController :type Controller%20Object%20Reference))
  (CallFunction|ChangeMappingContest true))

(event Input|EnhancedActionEvents|EnhancedInputActionIA_Back
  (params (ActionValue :type Boolean) (ElapsedSeconds :type Float%20%28double-precision%29) (TriggeredSeconds :type Float%20%28double-precision%29) (InputAction :type Input%20Action%20Object%20Reference :default "/Game/Inputs/Keypad/IA_Back.IA_Back"))
  (:Started
    (CallFunction|ExitKeypad)))

(event Input|EnhancedActionEvents|EnhancedInputActionIA_Right
  (params (ActionValue :type Boolean) (ElapsedSeconds :type Float%20%28double-precision%29) (TriggeredSeconds :type Float%20%28double-precision%29) (InputAction :type Input%20Action%20Object%20Reference :default "/Game/Inputs/Keypad/IA_Right.IA_Right"))
  (:Started
    (CallFunction|ChangeButtonHighlight (Variables|Data|GetCurrent%20Button) false)
    (bind _result (Math|Integer|IncrementInt (Variables|Data|GetCurrent%20Button))
      (:%20%20
        (if (== _result (Utilities|Array|Length (Variables|Data|GetButton%20list)))
          (Variables|Data|SetCurrent%20Button 0))
        (CallFunction|ChangeButtonHighlight (Variables|Data|GetCurrent%20Button) true)))))

(event Input|EnhancedActionEvents|EnhancedInputActionIA_Left
  (params (ActionValue :type Boolean) (ElapsedSeconds :type Float%20%28double-precision%29) (TriggeredSeconds :type Float%20%28double-precision%29) (InputAction :type Input%20Action%20Object%20Reference :default "/Game/Inputs/Keypad/IA_Left.IA_Left"))
  (:Started
    (CallFunction|ChangeButtonHighlight (Variables|Data|GetCurrent%20Button) false)
    (bind _result (Math|Integer|DecrementInt (Variables|Data|GetCurrent%20Button))
      (:%20%20
        (if (>= _result 0)
          _
          (else
            (bind _result_2 (Math|Integer|DecrementInt (Utilities|Array|Length (Variables|Data|GetButton%20list)))
              (:%20%20
                (Variables|Data|SetCurrent%20Button _result_2)))))
        (CallFunction|ChangeButtonHighlight (Variables|Data|GetCurrent%20Button) true)))))

(event Input|EnhancedActionEvents|EnhancedInputActionIA_Down
  (params (ActionValue :type Boolean) (ElapsedSeconds :type Float%20%28double-precision%29) (TriggeredSeconds :type Float%20%28double-precision%29) (InputAction :type Input%20Action%20Object%20Reference :default "/Game/Inputs/Keypad/IA_Down.IA_Down"))
  (:Started
    (CallFunction|ChangeButtonHighlight (Variables|Data|GetCurrent%20Button) false)
    (bind _output_get (Variables|Data|SetCurrent%20Button (+ (Variables|Data|GetCurrent%20Button) (Variables|Settings|GetButtonPerRow))))
    (if (< _output_get (Utilities|Array|Length (Variables|Data|GetButton%20list)))
      _
      (else
        (Variables|Data|SetCurrent%20Button (- (Variables|Data|GetCurrent%20Button) (Utilities|Array|Length (Variables|Data|GetButton%20list))))))
    (CallFunction|ChangeButtonHighlight (Variables|Data|GetCurrent%20Button) true)))

(event Input|EnhancedActionEvents|EnhancedInputActionIA_Up
  (params (ActionValue :type Boolean) (ElapsedSeconds :type Float%20%28double-precision%29) (TriggeredSeconds :type Float%20%28double-precision%29) (InputAction :type Input%20Action%20Object%20Reference :default "/Game/Inputs/Keypad/IA_Up.IA_Up"))
  (:Started
    (CallFunction|ChangeButtonHighlight (Variables|Data|GetCurrent%20Button) false)
    (bind _output_get (Variables|Data|SetCurrent%20Button (- (Variables|Data|GetCurrent%20Button) (Variables|Settings|GetButtonPerRow))))
    (if (>= _output_get 0)
      _
      (else
        (Variables|Data|SetCurrent%20Button (+ (Variables|Data|GetCurrent%20Button) (Utilities|Array|Length (Variables|Data|GetButton%20list))))))
    (CallFunction|ChangeButtonHighlight (Variables|Data|GetCurrent%20Button) true)))

(event Input|EnhancedActionEvents|EnhancedInputActionIA_Interact
  (params (ActionValue :type Boolean) (ElapsedSeconds :type Float%20%28double-precision%29) (TriggeredSeconds :type Float%20%28double-precision%29) (InputAction :type Input%20Action%20Object%20Reference :default "/Game/Inputs/Playerinput/IA_Interact.IA_Interact"))
  (bind _levelsequence (Variables|Data|GetLevelSequence))
  (bind _button_list (Variables|Data|GetButton%20list))
  (bind _current_button (Variables|Data|GetCurrent%20Button))
  (bind _output (Utilities|Array|Get(acopy) _button_list _current_button))
  (bind _buttoncontent (Variables|/Game/Bllueprints/Components/BPC_KeypadButton.BPC_KeypadButton_C|GetButtonContent _output))
  (:Started
    (CallFunction|AnimatePress)
    (switch string _buttoncontent
      (:Default
        (Class|FMODBlueprintStatics|PlayEvent2D "/Game/FMOD/Events/Keypad/ui-button-metal-button-spring-push-03.ui-button-metal-button-spring-push-03")
        (if (< (Utilities|String|Len (Variables|Settings|GetCurrent%20Code)) (Variables|Settings|GetMax%20Code%20Length))
          (bind _output_get (Variables|Settings|SetCurrent%20Code (Utilities|String|Append (Variables|Settings|GetCurrent%20Code) _buttoncontent)))
          (Rendering|Components|TextRender|SetText (Variables|Default|GetTXT_CurrentCode) (Utilities|Text|ToText(String) _output_get))))
      (:Confirm
        (if (Utilities|Enum|Equal(Enum) (Variables|Settings|GetCurrent%20Code) (Variables|settings|GetWanted%20Code))
          (Rendering|Components|TextRender|SetTextRenderColor (Variables|Default|GetTXT_CurrentCode) (Class|KismetMathLibrary|LinearColortoRGBE "(R=0.043050,G=0.359375,B=0.122131,A=1.000000)"))
          (CallFunction|ExitKeypad)
          (Variables|Data|SetIs%20Interactable false)
          (Utilities|FlowControl|Sequence
            (:then_0
              (Utilities|IsValid _levelsequence
                (:Is%20Valid
                  (Sequencer|Player|Play (Variables|/Script/LevelSequence.LevelSequenceActor|GetSequencePlayer _levelsequence) :!class /Script/MovieScene.MovieSceneSequencePlayer)))))
          (else
            (Rendering|Components|TextRender|SetTextRenderColor (Variables|Default|GetTXT_CurrentCode) (Class|KismetMathLibrary|LinearColortoRGBE "(R=0.987000,G=0.000000,B=0.097824,A=1.000000)"))
            (Input|DisableInput 0)
            (Utilities|FlowControl|Delay 0.5)
            (Utilities|RemoveCode)
            (Input|EnableInput 0))))
      (:Cancel
        (Utilities|RemoveCode)))))

(fn ConstructionScript
  (Variables|Data|SetButton%20list (Utilities|Array|MakeArray (Variables|Default|GetBPC_KeypadButton1) (Variables|Default|GetBPC_KeypadButton2) (Variables|Default|GetBPC_KeypadButton3) (Variables|Default|GetBPC_KeypadButton4) (Variables|Default|GetBPC_KeypadButton5) (Variables|Default|GetBPC_KeypadButton6) (Variables|Default|GetBPC_KeypadButto7) (Variables|Default|GetBPC_KeypadButton8) (Variables|Default|GetBPC_KeypadButton9) (Variables|Default|GetBPC_KeypadButton#1) (Variables|Default|GetBPC_KeypadButton) (Variables|Default|GetBPC_KeypadButton#2))))

(fn ChangeMappingContest
  (params (Condition :type Boolean))
  (bind _returnvalue (Game|GetPlayerController 0))
  (bind _returnvalue_2 (Game|GetPlayerController 0))
  (bind _returnvalue_3 (PlayerController|LocalPlayerSubsystems|GetEnhancedInputLocalPlayerSubsystem _returnvalue))
  (bind _returnvalue_4 (PlayerController|LocalPlayerSubsystems|GetEnhancedInputLocalPlayerSubsystem _returnvalue_2))
  (if Condition
    (Utilities|IsValid _returnvalue_3
      (:Is%20Valid
        (Input|RemoveMappingContext _returnvalue_3 "/Game/Inputs/Keypad/IMC_Keypad.IMC_Keypad" "(bIgnoreAllPressedKeysUntilRelease=True,bForceImmediately=False,bNotifyUserSettings=False)")))
    (else
      (Utilities|IsValid _returnvalue_4
        (:Is%20Valid
          (Input|AddMappingContext _returnvalue_4 "/Game/Inputs/Keypad/IMC_Keypad.IMC_Keypad" 0 "(bIgnoreAllPressedKeysUntilRelease=True,bForceImmediately=False,bNotifyUserSettings=False)"))))))

(fn IsInteractable
  (return (Variables|Data|GetIs%20Interactable)))